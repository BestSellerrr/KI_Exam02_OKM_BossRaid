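; Boss troll Blueprint that tracks health and turns into a ragdoll on death.
; BeginPlay fills health to max, and AnyDamage subtracts damage through SetHealth.
; SetHealth stores the value, prints it as debug text and fires the OnHealthChanged dispatcher for listeners.
; At zero or below, the mesh switches to the Ragdoll collision profile and starts simulating physics.
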(event `self.ReceiveBeginPlay`
  (`self.SetHealth` (`self.Health_Max`)))

(event `self.ReceiveAnyDamage`
  (params (Damage :type "Float (single-precision)") (DamageType :type "DamageType Object Reference") (InstigatedBy :type "Controller Object Reference") (DamageCauser :type "Actor Object Reference"))
  (bind _mesh (`self.Mesh`))
  (`self.SetHealth` (- (`self.Health_Current`) Damage))
  (if (<= (`self.Health_Current`) 0.0)
    (`PrimitiveComponent.SetCollisionProfileName` _mesh "Ragdoll" true)
    (`PrimitiveComponent.SetSimulatePhysics` _mesh true)))

(fn `SetHealth`
  (params (InHealth :type "Float (double-precision)"))
  (bind _output_get (set `self.Health_Current` InHealth))
  (`KismetSystemLibrary.PrintString` (`KismetStringLibrary.Conv_DoubleToString` _output_get))
  (`self.OnHealthChanged` _output_get))

(fn `UserConstructionScript`)