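; BP_Boss_Troll is a troll boss actor that tracks its health and handles its own death.
; BeginPlay and AnyDamage both route through SetHealth, which stores the new value and broadcasts OnHealthChanged.
; At zero health or below, the mesh switches to a simulated ragdoll and the actor is destroyed after a short delay.
; GetLocation supplies a random reachable navigation point within MoveRadius of the boss.
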(event `self.ReceiveBeginPlay`
  (`|ExecutionSequence`
    (:`then_0`
      (`self.SetHealth` (`self.Health_Max`)))))

(event `self.ReceiveAnyDamage`
  (params (Damage :type "Float (single-precision)") (DamageType :type "DamageType Object Reference") (InstigatedBy :type "Controller Object Reference") (DamageCauser :type "Actor Object Reference"))
  (bind _mesh (`self.Mesh`))
  ; 보스가 피격시 입은 데미지 계산
  (`self.SetHealth` (- (`self.Health_Current`) Damage))
  ; 보스 사망시 Ragdoll설정 및 일정 시간 이후 액터 삭제
  (if (<= (`self.Health_Current`) 0.0)
    (`PrimitiveComponent.SetCollisionProfileName` _mesh "Ragdoll" true)
    (`PrimitiveComponent.SetSimulatePhysics` _mesh true)
    (`KismetSystemLibrary.Delay` 3.0)
    (`self.K2_DestroyActor`)))

(fn `GetLocation`
  (returns (OutLocation :type "Vector Structure"))
  (return (`NavigationSystemV1.K2_GetRandomReachablePointInRadius` (`self.K2_GetActorLocation`) (`self.Move_Radius`) null null)))

(fn `SetHealth`
  (params (InHealth :type "Float (double-precision)"))
  (bind _output_get (set `self.Health_Current` InHealth))
  (`self.OnHealthChanged` _output_get))

(fn `UserConstructionScript`)